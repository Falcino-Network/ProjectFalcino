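; BP_Terminal is an interactable terminal actor that presents a screen UI to the third-person character.
; Entering and leaving its ActivationPoint sets the in-range player and calls a shared FlipFlop toggle that creates or removes the Terminal_UI widget, hiding the cursor on removal.
; Interact, when in range, locks the player, shows the cursor, reveals the terminal and sets it up with ScreenDetails.
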(event OnComponentBeginOverlap(ActivationPoint)
  (params (OverlappedComponent :type Primitive%20Component%20Object%20Reference) (OtherActor :type Actor%20Object%20Reference) (OtherComp :type Primitive%20Component%20Object%20Reference) (OtherBodyIndex :type Integer) (bFromSweep :type Boolean) (SweepResult :type Hit%20Result%20Structure%20%28by%20ref%29))
  ;[1 1 1] Activate Terminal Space
  (bind _asbp_third_person_character (Utilities|Casting|CastToBP_ThirdPersonCharacter OtherActor))
  (Variables|Default|SetIsInRange true)
  (Variables|Default|SetPlayer _asbp_third_person_character)
  (CallFunction|ToggleTerminal))

(event OnComponentEndOverlap(ActivationPoint)
  (params (OverlappedComponent :type Primitive%20Component%20Object%20Reference) (OtherActor :type Actor%20Object%20Reference) (OtherComp :type Primitive%20Component%20Object%20Reference) (OtherBodyIndex :type Integer))
  ;[1 1 1] Activate Terminal Space
  (Utilities|Casting|CastToBP_ThirdPersonCharacter OtherActor)
  (Variables|Default|SetIsInRange false)
  (Variables|Default|SetPlayer 0)
  (CallFunction|ToggleTerminal))

(event Custom|ToggleTerminal
  (bind _returnvalue (Game|GetPlayerController 0))
  ;[1 1 1] Toggle Terminal
  (Utilities|FlowControl|FlipFlop
    (:A
      (bind _returnvalue_2 (UserInterface|CreateWidget "/Game/FalcinoHUD/UI/Terminal_UI.Terminal_UI_C" _returnvalue))
      (bind _output_get (Variables|Default|SetTerminalUI _returnvalue_2))
      (UserInterface|Viewport|AddtoViewport _output_get 0))
    (:B
      (Variables|/Script/Engine.PlayerController|SetbShowMouseCursor _returnvalue false)
      (Widget|RemovefromParent (Variables|Default|GetTerminalUI))
      (Variables|Default|SetTerminalUI 0))))

(event EventInteract
  (bind _terminalui (Variables|Default|GetTerminalUI))
  ;[1 1 1] Interact
  (if (Variables|Default|GetIsInRange)
    (Default|LockPlayer (Variables|Default|GetPlayer))
    (Variables|/Script/Engine.PlayerController|SetbShowMouseCursor (Game|GetPlayerController 0) true)
    (Default|ShowTerminal _terminalui)
    (Default|Setup _terminalui (Variables|Default|GetScreenDetails))))

(fn ConstructionScript)